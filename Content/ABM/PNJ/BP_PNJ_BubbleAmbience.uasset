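; NPC ambient bubble Blueprint that shows random lines in a WBP_AmbientBubble widget while the player is flagged in range.
; BeginPlay hides the widget and caches lines from a data table row.
; Externally callable Start/StopAmbientLoop functions control a looping timer, its interval randomized once per start.
; Each attempt avoids repeating the last line, requires at least two lines, skips busy widgets, and starts a cooldown after playing.
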(event `self.ReceiveBeginPlay`
  (bind _aswbp_ambient_bubble (cast `/Game/ABM/PNJ/Bulle_Ambiance/Widget/WBP_AmbientBubble` (`WidgetComponent.GetUserWidgetObject` (`self.WC_Bubble`))))
  (`Widget.SetVisibility` _aswbp_ambient_bubble "Collapsed")
  (`self.LoadAmbientLines`))

(event `ResetCooldown`
  (set `self.bOnCooldown` false))

(event `AmbientLoopTick`
  (if (`self.bPlayerInRange`)
    (`self.PlayRandomAmbientLine`)))

(fn `LoadAmbientLines`
  (if (`KismetSystemLibrary.IsValid` (`self.AmbiantDataTable`))
    (bind _returnvalue (`|GetDataTableRow` (`self.AmbiantDataTable`) (`self.Row Name`))
      (:`then`
        (set `self.LinesCache` (`.MemberVar_0_2_8C37DB0844CDD3B8D02461BFFD2FB4A9` (break `/Game/ABM/PNJ/Bulle_Ambiance/Data/ST_AmbientLineRow` _returnvalue))))
      (:`RowNotFound`
        (return)))
    (else
      (return))))

(fn `PlayRandomAmbientLine`
  (bind _returnvalue (`KismetArrayLibrary.Array_Length` (`self.LinesCache`)))
  (bind _returnvalue_2 (`KismetMathLibrary.RandomIntegerInRange` 0 (- _returnvalue 1)))
  (if (`self.bBubbleEnable`)
    (if (not (`self.bOnCooldown`))
      (if (> _returnvalue 0)
        (if (> _returnvalue 1) :!label _label
          (if (== (`self.LastLineIndex`) _returnvalue_2)
            (goto _label)
            (else
              (set `self.LastLineIndex` _returnvalue_2)
              (bind _aswbp_ambient_bubble (cast `/Game/ABM/PNJ/Bulle_Ambiance/Widget/WBP_AmbientBubble` (`WidgetComponent.GetUserWidgetObject` (`self.WC_Bubble`))))
              (if (not (`/Game/ABM/PNJ/Bulle_Ambiance/Widget/WBP_AmbientBubble.bIsBusy` _aswbp_ambient_bubble))
                (`/Game/ABM/PNJ/Bulle_Ambiance/Widget/WBP_AmbientBubble.PlayLine` _aswbp_ambient_bubble (`|GetArrayItem` (`self.LinesCache`) (`self.LastLineIndex`)))
                (set `self.bOnCooldown` true)
                (`KismetSystemLibrary.K2_ClearAndInvalidateTimerHandle` (`self.CoolDownTimer`))
                (bind _returnvalue_3 (`KismetSystemLibrary.K2_SetTimerDelegate` (`|CreateDelegate` :!event `ResetCooldown`) (`self.BubbleCooldownTime`)))
                (set `self.CoolDownTimer` _returnvalue_3)))))
        (else
          (return))))
    (else
      (return))))

(fn `StartAmbientLoop`
  (if (`self.bBubbleEnable`)
    (set `self.bPlayerInRange` true)
    (`KismetSystemLibrary.K2_ClearAndInvalidateTimerHandle` (`self.AmbientLoopTimer`))
    (`self.PlayRandomAmbientLine`)
    (bind _returnvalue (`KismetSystemLibrary.K2_SetTimerDelegate` (`|CreateDelegate` :!event `AmbientLoopTick`) (`KismetMathLibrary.RandomFloatInRange` (`self.MinAmbientInterval`) (`self.MaxAmbientInterval`)) true))
    (set `self.AmbientLoopTimer` _returnvalue)
    (return)
    (else
      (return))))

(fn `StopAmbientLoop`
  (set `self.bPlayerInRange` false)
  (`KismetSystemLibrary.K2_ClearAndInvalidateTimerHandle` (`self.AmbientLoopTimer`))
  (return))

(fn `UserConstructionScript`)