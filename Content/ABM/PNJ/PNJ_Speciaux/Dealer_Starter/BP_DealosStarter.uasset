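; BP_DealosStarter is a special NPC that lets the player pick a starter mask through dialogue.
; When dialogue ends with an event pending, it puts the player controller in choice mode and spawns three BP_StarterMask actors as selectable options.
; A selection stores the choice and advances the dialogue.
; The next dialogue end gives the mask once, applies the chosen material to the player mesh and exits the sequence.
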(event `OnChoiceSelected`
  (params (ChoiceId :type Integer))
  (set `self.Choice Id` ChoiceId)
  (set `self.bHaveEventDuring?` false)
  (`self.AdvanceDialogue`))

(event `self.OnDialogueEnd`
  (params (PlayerCharacter :type "/Game/ABM/Core/Character/BP_ThirdPersonCharacter Object Reference"))
  (if (`self.bHaveEventDuring?`)
    (`self.BeginChoicePhase`)
    (else
      (`/Engine/EditorBlueprintResources/StandardMacros.DoOnce` false
        (:`Completed`
          (`/Game/ABM/Mask_System/Add_Component/BP_AC_MaskState.SetMask` (`/Game/ABM/Core/Character/BP_ThirdPersonCharacter.BP_AC_MaskState` PlayerCharacter) (`self.MaskGive`))
          (`PrimitiveComponent.SetMaterial` (`Character.Mesh` PlayerCharacter) 1 (`|GetArrayItem` (`self.Mask Material `) (`self.Choice Id`)))
          (`self.ExitDialogueSequence`))))))

(event `BeginChoicePhase`
  (bind _asbp_third_person_player_controller (cast `/Game/ThirdPerson/Blueprints/BP_ThirdPersonPlayerController` (`GameplayStatics.GetPlayerController` 0)))
  (bind _output_get (set `self.As BP Third Person Player Controller` _asbp_third_person_player_controller))
  (`/Game/ThirdPerson/Blueprints/BP_ThirdPersonPlayerController.EnterChoiceMode` _output_get self)
  (for _index (range 3)
    (bind _returnvalue (`|SpawnActorFromClass` "/Game/ABM/PNJ/PNJ_Speciaux/Dealer_Starter/BP_StarterMask.BP_StarterMask_C" (`SceneComponent.K2_GetComponentToWorld` (select `int` _index :`0` (`self.P0`) :`1` (`self.P1`) :`2` (`self.P2`))) "Undefined" "MultiplyWithRoot" null _index (`|GetArrayItem` (`self.Mask Material `) _index) null))
    (`KismetArrayLibrary.Array_AddUnique` (`/Game/ThirdPerson/Blueprints/BP_ThirdPersonPlayerController.ChoiceActors` (`self.As BP Third Person Player Controller`)) _returnvalue)))

(fn `UserConstructionScript`
  (`parent.UserConstructionScript`))