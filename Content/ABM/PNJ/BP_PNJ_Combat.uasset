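; NPC fighter AI for side-view combat against the player, with movement along Y and X locked by timer.
; StartFight begins a randomly delayed decision loop choosing between approaching, punching, jumping high kicks and fleeing or dashing, using distance and weighted randomness.
; Montage notifies trigger line-trace hits that apply damage and launch knockback.
; Taking damage plays camera shake, FMOD sound and hit stop through zeroed time dilation with mesh jitter.
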(event `self.ReceiveBeginPlay`
  (bind _returnvalue_x (`KismetMathLibrary.BreakVector` (`self.K2_GetActorLocation`)))
  (set `self.ForceXLoc` _returnvalue_x)
  (set `self.BaseRelativeLoc` (`SceneComponent.RelativeLocation` (`self.Mesh`))))

(event `StartFight`
  (set `self.CharaState` "NewEnumerator1")
  (set `self.bContinueFight?` true)
  (bind _returnvalue (`GameplayStatics.GetActorOfClass` "/Game/ABM/Core/Character/BP_ThirdPersonCharacter.BP_ThirdPersonCharacter_C"))
  (set `self.RefChara` _returnvalue)
  (`self.Analyse`)
  (`KismetSystemLibrary.K2_SetTimer` null "UpdateXAxe" 0.01 true true))

(event `Loose`
  ; TO DO : Chara LOOSE disapear ?
  (set `self.bContinueFight?` false)
  (set `self.CharaState` "NewEnumerator0"))

(event `Analyse`
  (if (`self.bContinueFight?`)
    ; Time to analyse
    (`KismetSystemLibrary.Delay` (`KismetMathLibrary.RandomFloatInRange` 0.25 0.75))
    ; Look where is the player
    (if (`self.CheckDistanceOnAxe` (`self.HighKickDistance`))
      (if (`KismetMathLibrary.RandomBoolWithWeight` 0.4)
        (`self.DirectAttack`)
        (else
          (`self.CloseRangeAndTryAttack`)))
      (elif (`KismetMathLibrary.RandomBoolWithWeight` 0.3)
        (`self.Flee`)
        (else
          (`self.CloseRangeAndTryAttack`))))))

(event `Punch`
  ; Sometime make some fake high kick
  (if (not (`KismetMathLibrary.RandomBoolWithWeight` 0.8))
    (set `CharacterMovementComponent.JumpZVelocity` 100.0 (`self.CharacterMovement`))
    (`self.Jump`))
  (`self.RotateToAttack`)
  ; Anim and shot
  (bind _punchanim (`self.PunchAnim`)
    (:`then`
      (bind _notifyname (`|PlayMontage` (`self.Mesh`) _punchanim (`self.PlayRate`))
        (:`OnCompleted`
          (`self.Analyse` :!label _label))
        (:`OnInterrupted`
          (goto _label))
        (:`OnNotifyBegin`
          (switch `name` _notifyname
            (:`Punch`
              (`self.ApplyDamageIfTouch` (`self.PunchDistance`) (`KismetMathLibrary.RandomFloatInRange` (`self.PunchDamage`) 2.0) 500.0 300.0 :!label _label_2))))))
    (:`else`
      (`|ExecutionSequence`
        (:`then_0`
          (goto _label_2))
        (:`then_1`
          (goto _label))))))

(event `HighKick`
  ; Sometime make some fake high kick
  (if (`KismetMathLibrary.RandomBoolWithWeight` 0.6)
    (set `CharacterMovementComponent.JumpZVelocity` 500.0 (`self.CharacterMovement`))
    (`self.Jump`)
    (`KismetSystemLibrary.Delay` 0.2)
    (`self.RotateToAttack`)
    ; Anim and shot
    (bind _highkickanim (`self.HighKickAnim`)
      (:`then`
        (bind _notifyname (`|PlayMontage` (`self.Mesh`) _highkickanim (`self.PlayRate`))
          (:`OnCompleted`
            (`self.Analyse` :!label _label_3))
          (:`OnInterrupted`
            (goto _label_3))
          (:`OnNotifyBegin`
            (switch `name` _notifyname
              (:`Kick`
                (`self.ApplyDamageIfTouch` (`self.HighKickDistance`) (`KismetMathLibrary.RandomFloatInRange` (`self.HighKickDamage`) 3.0) 1000.0 :!label _label_4))))))
      (:`else`
        (`|ExecutionSequence`
          (:`then_0`
            (goto _label_4))
          (:`then_1`
            (goto _label_3)))))
    (else
      (set `CharacterMovementComponent.JumpZVelocity` 100.0 (`self.CharacterMovement`))
      (`self.Jump`)
      (`self.RotateToAttack`)
      (`self.Punch`))))

(event `Flee`
  (bind (_closedistance _flee) (`self.getNormalizeDirFromChara`))
  (if (`self.bContinueFight?`)
    (if (`KismetMathLibrary.RandomBoolWithWeight` 0.6)
      (`self.GenerateRndValueToFlee`)
      (if (>= (`self.GeneratedRndValue`) 590.0)
        ; Have see he can't flee true try punch else he try but failed
        (if (`KismetMathLibrary.RandomBool`)
          (if (`KismetMathLibrary.RandomBoolWithWeight` 0.6)
            (`self.Punch`)
            (else
              (`self.HighKick`)))
          (else
            (`|AIMoveTo` self (`self.getLocToFlee`) null (`self.AttackRange`) :!label _label_5
              (:`OnSuccess`
                (`self.CloseRangeAndTryAttack`))
              (:`OnFail`
                ; If chara close Flee if chara far close the distance and try attacking
                (`self.Dash` _closedistance :!label _label_6)
                (`self.DirectAttack`)))))
        (else
          (goto _label_5)))
      (elif (< (`KismetMathLibrary.Vector_Distance` (`self.K2_GetActorLocation` (`self.RefChara`)) (`self.K2_GetActorLocation`)) 200.0)
        (`self.Dash` _flee)
        (`self.DirectAttack`)
        (else
          (goto _label_6))))))

(event `Dash`
  (params (DashSens :type "Float (double-precision)"))
  (`self.LaunchCharacter` (`KismetMathLibrary.MakeVector` 0.0 (* DashSens 1000.0) 200.0) true))

(event `self.ReceiveAnyDamage`
  (params (Damage :type "Float (single-precision)") (DamageType :type "DamageType Object Reference") (InstigatedBy :type "Controller Object Reference") (DamageCauser :type "Actor Object Reference"))
  ; HIT STOP
  (`GameplayStatics.PlayWorldCameraShake` "/Game/ABM/Core/Shake/BP_HitCameraShake.BP_HitCameraShake_C" (`self.K2_GetActorLocation`) 500.0 20000.0)
  (`FMODBlueprintStatics.PlayEvent2D` (`self.FMOD_Hit`))
  (`self.StartHitStop` 0.2 true)
  (`TimelineComponent.SetPlayRate` (`self.HitStop`) (/ 1.0 0.5))
  (`TimelineComponent.SetPlayRate` (`self.HitStopReturn`) (/ 1.0 0.5)))

(event `CloseRangeAndTryAttack`
  (if (`self.bContinueFight?`)
    (set `self.AttackRange` (`KismetMathLibrary.RandomFloatInRange` 50.0 (`self.HighKickDistance`)))
    (`|AIMoveTo` self (0.0 0.0 0.0) (`self.RefChara`) (`self.AttackRange`)
      (:`OnSuccess`
        (`self.DirectAttack`))
      (:`OnFail`
        (`self.CloseRangeAndTryAttack`)))))

(fn `ApplyDamageIfTouch`
  (params (Distance :type "Float (single-precision)") (BaseDamage :type "Float (single-precision)") (KnockbackForce :type "Float (double-precision)" :default 500.0) (KnockbackHeight :type "Float (double-precision)" :default 200.0))
  (returns (DamageDealed :type "Float (single-precision)"))
  (bind (_returnvalue _outhit) (`self.LineTrace` (`local.Distance`)))
  (bind (_bblockinghit _binitialoverlap _time _distance _location _impactpoint _normal _impactnormal _physmat _hitactor) (`GameplayStatics.BreakHitResult` _outhit))
  (if (and _returnvalue (`KismetSystemLibrary.IsValid` _hitactor))
    (if (< (.y (`self.GetVelocity` (`self.RefChara`))) -5.0)
      (return 0.0)
      (else
        (bind _returnvalue_2 (`GameplayStatics.ApplyDamage` _hitactor (`local.BaseDamage`)))
        (`self.KnockBack` (cast `Character` _hitactor :!pure true) (`KismetMathLibrary.MakeVector` 0.0 (.y (* (`KismetMathLibrary.Normal` (- (`self.K2_GetActorLocation` _hitactor) (`self.K2_GetActorLocation`))) (`local.KnockbackForce`))) (`local.KnockbackHeight`)))
        (return _returnvalue_2)))
    (else
      (return 0.0))))

(fn `CheckDistanceOnAxe`
  (params (Distance :type "Float (double-precision)"))
  (returns (ReturnValue :type Boolean))
  (return (> (`KismetMathLibrary.Abs` (- (`self.getPlayerLocOnAxe`) (`self.getActorAxe`))) Distance)))

(fn `DirectAttack`
  (if (`self.getDistanceFromActorIsLessThan` (`self.PunchDistance`))
    (`self.Punch`)
    (elif (`self.getDistanceFromActorIsLessThan` (`self.HighKickDistance`))
      (`self.HighKick`)
      (else
        (switch `int` (`KismetMathLibrary.RandomIntegerInRange` 0 2) ; else random strategy
          (:`Default`
            (`self.Flee` :!label _label))
          (:`0`
            (`self.Punch`))
          (:`1`
            (`self.HighKick`))
          (:`2`
            (goto _label)))))))

(fn `EndHitStop`
  (set `self.CustomTimeDilation` 1.0)
  (`KismetSystemLibrary.K2_ClearTimer` null "ShakeSpriteHorizontal")
  (`KismetSystemLibrary.K2_ClearTimer` null "ShakeSpriteVertical"))

(fn `GenerateRndValueToFlee`
  (bind _fightmanager (`self.FightManager`))
  (bind _y (`self.getAxe` (`/Game/ABM/Core/Blueprints/MiniGame/Fight/BP_FightingMiniGameManager.RightBox` _fightmanager)))
  (set `self.GeneratedRndValue` (`KismetMathLibrary.RandomFloatInRange` (`KismetMathLibrary.FClamp` (+ (`self.getPlayerLocOnAxe`) 100.0) (`self.getAxe` (`/Game/ABM/Core/Blueprints/MiniGame/Fight/BP_FightingMiniGameManager.LeftBox` _fightmanager)) _y) _y)))

(fn `getActorAxe`
  (returns (Y :type "Float (double-precision)"))
  (return (.y (`self.K2_GetActorLocation`))))

(fn `getAxe`
  (params (SceneComp :type "SceneComponent Object Reference"))
  (returns (Y :type "Float (double-precision)"))
  (return (.y (`SceneComponent.K2_GetComponentLocation` SceneComp))))

(fn `GetCharaForAnimState`
  (returns (CharaState :type "/Game/ABM/Core/Library/E_CharaStatesPossible Enum"))
  (return (`self.CharaState`)))

(fn `getDistanceFromActorIsLessThan`
  (params (Distance :type "Float (double-precision)"))
  (returns (ReturnValue :type Boolean))
  (return (< (`KismetMathLibrary.Vector_Distance` (`self.K2_GetActorLocation` (`self.RefChara`)) (`self.K2_GetActorLocation`)) Distance)))

(fn `getLocToFlee`
  (returns (ReturnValue :type "Vector Structure"))
  (return (`KismetMathLibrary.MakeVector` (.x (`self.K2_GetActorLocation`)) (`self.GeneratedRndValue`) (.z (`self.K2_GetActorLocation`)))))

(fn `getNormalizeDirFromChara`
  (returns (CloseDistance :type "Float (double-precision)") (Flee :type "Float (double-precision)"))
  (return (.y (`KismetMathLibrary.Normal` (- (`self.K2_GetActorLocation` (`self.RefChara`)) (`self.K2_GetActorLocation`)))) (.y (`KismetMathLibrary.Normal` (- (`self.K2_GetActorLocation`) (`self.K2_GetActorLocation` (`self.RefChara`)))))))

(fn `getPlayerLocOnAxe`
  (returns (Y :type "Float (double-precision)"))
  (return (.y (`self.K2_GetActorLocation` (`self.RefChara`)))))

(fn `KnockBack`
  (params (Target :type "Character Object Reference") (LaunchVelocity :type "Vector Structure"))
  (`/Engine/EditorBlueprintResources/StandardMacros.IsValid` Target
    (:`Is Valid`
      (`self.LaunchCharacter` Target LaunchVelocity true true))))

(fn `LineTrace`
  (params (Distance :type "Float (single-precision)"))
  (returns (ReturnValue :type Boolean) (OutHit :type "HitResult Structure"))
  (bind _returnvalue (`self.K2_GetActorLocation`))
  (bind (_returnvalue_x _returnvalue_y _returnvalue_z) (`KismetMathLibrary.BreakVector` (`SceneComponent.K2_GetComponentScale` (`self.Mesh`))))
  (bind (_outhit _returnvalue_2) (`KismetSystemLibrary.LineTraceSingleForObjects` :`Start` (+ _returnvalue (0.0 0.0 -25.0)) :`End` (+ (+ _returnvalue (* (`SceneComponent.GetForwardVector` (`self.Mesh`)) (`local.Distance`) _returnvalue_z)) (0.0 0.0 -25.0)) :`ObjectTypes` (`|MakeArray` "ObjectTypeQuery3" :!type "EObjectTypeQuery Enum") :`DrawDebugType` (`self.LineTraceDrawDebug`)))
  (return _returnvalue_2 _outhit))

(fn `RotateToAttack`
  (`SceneComponent.SetRelativeScale3D` (`self.Mesh`) (`KismetMathLibrary.MakeVector` (`KismetMathLibrary.SelectFloat` 1.0 -1.0 (>= (.x (`KismetMathLibrary.Normal` (- (`self.K2_GetActorLocation` (`self.RefChara`)) (`self.K2_GetActorLocation`)))) 0.0)) 1.0 1.0)))

(fn `ShakeSpriteHorizontal`
  (bind (_baserelativeloc_x _baserelativeloc_y _baserelativeloc_z) (`KismetMathLibrary.BreakVector` (`self.BaseRelativeLoc`)))
  (bind _isa (`/Engine/EditorBlueprintResources/StandardMacros.FlipFlop`)
    (:`A`
      _)
    (:`B`
      _))
  (`SceneComponent.K2_SetRelativeLocation` (`self.Mesh`) (`KismetMathLibrary.MakeVector` _baserelativeloc_x (+ _baserelativeloc_y (select `bool` _isa :`false` (+ (`self.SpriteShakeDistanceHor`) -1.0) :`true` (`self.SpriteShakeDistanceHor`) :!type "Float (single-precision)")) _baserelativeloc_z) false false))

(fn `ShakeSpriteVertical`
  (bind (_baserelativeloc_x _baserelativeloc_y _baserelativeloc_z) (`KismetMathLibrary.BreakVector` (`self.BaseRelativeLoc`)))
  (bind _isa (`/Engine/EditorBlueprintResources/StandardMacros.FlipFlop`)
    (:`A`
      _)
    (:`B`
      _))
  (`SceneComponent.K2_SetRelativeLocation` (`self.Mesh`) (`KismetMathLibrary.MakeVector` _baserelativeloc_x _baserelativeloc_y (+ _baserelativeloc_z (select `bool` _isa :`false` (+ (`self.SpriteShakeDistanceVer`) -1.0) :`true` (`self.SpriteShakeDistanceVer`) :!type "Float (single-precision)"))) false false))

(fn `StartHitStop`
  (params (Duration :type "Float (double-precision)") (`IsVictim?` :type Boolean))
  (set `self.CustomTimeDilation` 0.0)
  (`KismetSystemLibrary.K2_SetTimer` null "EndHitStop" Duration false false Duration)
  (if (`local.IsVictim?`)
    (`KismetSystemLibrary.K2_SetTimer` null "ShakeSpriteHorizontal" (`KismetMathLibrary.RandomFloatInRange` 0.015 0.025) true true)
    (`KismetSystemLibrary.K2_SetTimer` null "ShakeSpriteVertical" (`KismetMathLibrary.RandomFloatInRange` 0.015 0.025) true true)))

(fn `UpdateXAxe`
  (`self.K2_SetActorLocation` (`KismetMathLibrary.MakeVector` (`self.ForceXLoc`) (.y (`self.K2_GetActorLocation`)) (.z (`self.K2_GetActorLocation`)))))

(fn `UserConstructionScript`)