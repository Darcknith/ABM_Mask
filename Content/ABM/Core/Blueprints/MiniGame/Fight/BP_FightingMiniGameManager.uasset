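; Manager actor that runs the fighting minigame, with two side boxes that gain collision when it starts.
; Start blends the view to the assigned camera, shows a transition widget and glides the player onto the manager's position with a looping timer.
; After the fade, it adds BPC_FightingMiniGame to the player, whose fight-start event starts RefCharaFighter.
; End clears the running flag, re-arms the start and calls Loose on the fighter.
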(event `self.ReceiveBeginPlay`)

(event `OnFightStart`
  ;[0.15 0.7826 0.15 0.5] Fight Start
  (`/Game/ABM/PNJ/BP_PNJ_Combat.StartFight` (`self.RefCharaFighter`)))

(event `/Game/ABM/Core/Interfaces/BPI_MiniGame.MiniGameStart`
  ; Trigger maybe after a dialogue
  (message `/Game/ABM/Core/Interfaces/BPI_CameraManager.setTrack` (`GameplayStatics.GetPlayerCameraManager` 0) 5)
  (`/Engine/EditorBlueprintResources/StandardMacros.DoOnce` false :!label _label
    (:`Completed`
      (`self.setCollision` "QueryAndPhysics")
      (set `self.bGameIsRunning?` true)
      (bind _cameraref (`self.CameraRef`)
        (:`then`
          (`PlayerController.SetViewTargetWithBlend` (`GameplayStatics.GetPlayerController` 0) _cameraref (`self.BlendTime`) "VTBlend_Linear" 0.0 false)
          (`KismetSystemLibrary.K2_SetTimer` null "MoveActorToLocation" 0.001 true true)
          (bind _returnvalue (`|CreateWidget` "/Game/ABM/Widgets/Organismes/WBP_Transition.WBP_Transition_C" null 0.25 false 1.0 0.5))
          (add `/Game/ABM/Widgets/Organismes/WBP_Transition.WhenFinish` _returnvalue (`|CreateDelegate` :!event `WhenFadeIsFinished`))
          (add `/Game/ABM/Widgets/Organismes/WBP_Transition.WhenTimerOver` _returnvalue (`|CreateDelegate` :!event `TimerFadeOver`))
          (`UserWidget.AddToViewport` _returnvalue 0))
        (:`else`
          (`KismetSystemLibrary.PrintString` "BP_FightingMiniGameManager // NO CAMERA WAS SETUP" true false (struct :`G` 0.66 :`B` 1.0 :`A` 1.0) 5.0))))))

(event `/Game/ABM/Core/Interfaces/BPI_MiniGame.MiniGameEnd`
  (set `self.bGameIsRunning?` false)
  (`|ExecutionSequence`
    (:`then_0`
      (goto _label :!via `Reset`))
    (:`then_1`
      (`/Game/ABM/PNJ/BP_PNJ_Combat.Loose` (`self.RefCharaFighter`)))
    (:`then_2`
      (message `/Game/ABM/Core/Interfaces/BPI_CameraManager.setTrack` (`GameplayStatics.GetPlayerCameraManager` 0) 0))))

(event `WhenFadeIsFinished`
  (bind _returnvalue (`|AddComponentByClass` (`GameplayStatics.GetPlayerCharacter` 0) "/Game/ABM/Core/Blueprints/MiniGame/Fight/BPC_FightingMiniGame.BPC_FightingMiniGame_C"))
  (bind _output_get (set `self.RefComponent` _returnvalue))
  (`/Game/ABM/Core/Blueprints/MiniGame/Fight/BPC_FightingMiniGame.InitializeBPC` _output_get self)
  (add `/Game/ABM/Core/Blueprints/MiniGame/Fight/BPC_FightingMiniGame.FightStart` (`self.RefComponent`) (`|CreateDelegate` :!event `OnFightStart`)))

(event `TimerFadeOver`
  (bind (_returnvalue_x _returnvalue_y) (`KismetMathLibrary.BreakVector` (`self.K2_GetActorLocation`)))
  (`KismetSystemLibrary.K2_ClearTimer` null "MoveActorToLocation")
  (`self.K2_SetActorLocation` (`GameplayStatics.GetPlayerCharacter` 0) (`KismetMathLibrary.MakeVector` _returnvalue_x _returnvalue_y (.z (`self.K2_GetActorLocation` (`GameplayStatics.GetPlayerCharacter` 0)))) false false))

(fn `MoveActorToLocation`
  (bind (_returnvalue_x _returnvalue_y) (`KismetMathLibrary.BreakVector` (`self.K2_GetActorLocation`)))
  (`self.K2_SetActorLocation` (`GameplayStatics.GetPlayerCharacter` 0) (`KismetMathLibrary.VInterpTo` (`self.K2_GetActorLocation` (`GameplayStatics.GetPlayerCharacter` 0)) (`self.K2_GetActorLocation`) (`GameplayStatics.GetWorldDeltaSeconds`) 5.0) false false)
  (if (== (`KismetMathLibrary.MakeVector` (.x (`self.K2_GetActorLocation` (`GameplayStatics.GetPlayerCharacter` 0))) (.y (`self.K2_GetActorLocation` (`GameplayStatics.GetPlayerCharacter` 0)))) (`KismetMathLibrary.MakeVector` (.x (`self.K2_GetActorLocation`)) (.y (`self.K2_GetActorLocation`))) :`ErrorTolerance` 2.0)
    (`self.K2_SetActorLocation` (`GameplayStatics.GetPlayerCharacter` 0) (`KismetMathLibrary.MakeVector` _returnvalue_x _returnvalue_y (.z (`self.K2_GetActorLocation` (`GameplayStatics.GetPlayerCharacter` 0)))) false false)
    (`KismetSystemLibrary.K2_ClearTimer` null "MoveActorToLocation")))

(fn `setCollision`
  (params (NewType :type "ECollisionEnabled Enum" :default "NoCollision"))
  (`PrimitiveComponent.SetCollisionEnabled` (`self.LeftBox`) NewType)
  (`PrimitiveComponent.SetCollisionEnabled` (`self.RightBox`) NewType))

(fn `UserConstructionScript`
  (`BoxComponent.SetBoxExtent` (`self.RightBox`) (`self.In Box Extent`) true)
  (`BoxComponent.SetBoxExtent` (`self.LeftBox`) (`self.In Box Extent`) true)
  (`self.setCollision` "NoCollision")
  (`SceneComponent.K2_SetWorldLocation` (`self.LeftBox`) (+ (`self.LeftBoxLoc`) (`self.K2_GetActorLocation`)) false false)
  (`SceneComponent.K2_SetWorldLocation` (`self.RightBox`) (+ (`self.RightBoxLoc`) (`self.K2_GetActorLocation`)) false false))