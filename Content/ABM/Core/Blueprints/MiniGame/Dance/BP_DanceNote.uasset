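; BP_DanceNote is a moving directional note for the dance rhythm minigame.
; InitNote stores spawn and hit times, lowers both endpoints by a fixed Z offset, and rotates the Plane's yaw to match one of four directions.
; While active, Tick lerps the actor from start to target by game time, clamped so it stops at the target at hit time.
; Disconnected scaling logic never runs.
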(event `self.ReceiveTick`
  (params (DeltaSeconds :type "Float (single-precision)"))
  (if (`self.bActive`)
    (`self.K2_SetActorLocation` (`KismetMathLibrary.VLerp` (`self.StartLocation`) (`self.TargetLocation`) (`KismetMathLibrary.FClamp` (- 1.0 (/ (- (`self.HitTime`) (`KismetSystemLibrary.GetGameTimeInSeconds`)) (- (`self.HitTime`) (`self.SpawnTime`)))))))))

(fn `InitNote`
  (params (InStartLocation :type "Vector Structure") (InTargetLocation :type "Vector Structure") (InSpawnTime :type "Float (double-precision)") (InHitTime :type "Float (double-precision)") (InDirection :type Byte))
  (set `self.StartLocation` (`KismetMathLibrary.MakeVector` (.x InStartLocation) (.y InStartLocation) (- (.z InStartLocation) 80.0)))
  (set `self.TargetLocation` (`KismetMathLibrary.MakeVector` (.x InTargetLocation) (.y InTargetLocation) (- (.z InTargetLocation) 80.0)))
  (set `self.SpawnTime` InSpawnTime)
  (set `self.HitTime` InHitTime)
  (bind _output_get (set `self.Direction` InDirection))
  (set `self.bActive` true)
  (`self.K2_SetActorLocation` (`self.StartLocation`))
  (`SceneComponent.K2_SetWorldRotation` (`self.Plane`) (`KismetMathLibrary.MakeRotator` 0.0 0.0 (select `byte` _output_get :`0` -90.0 :`1` 0.0 :`2` 90.0 :`3` 180.0 :!type "Float (single-precision)")) false false))

(fn `UserConstructionScript`)