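; Rhythm dance minigame actor that spawns note actors toward the player and scores timed arrow-key presses.
; BuildNotes creates an evenly spaced chart with random directions on BeginPlay; StartMinigame opens the score widget and starts a looping timer.
; TickInGame spawns notes ahead of their hit times, flags late misses and stops at GameDuration.
; JudgeInput grades the closest unjudged same-direction note as Perfect, Good or Miss, updating score and combo.
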(event `Key|Up`
  (params (Key :type "Key Structure"))
  (:`Pressed`
    (`self.JudgeInput` 1)))

(event `Key|Left`
  (params (Key :type "Key Structure"))
  (:`Pressed`
    (`self.JudgeInput` 0)))

(event `Key|Right`
  (params (Key :type "Key Structure"))
  (:`Pressed`
    (`self.JudgeInput` 2)))

(event `Key|Down`
  (params (Key :type "Key Structure"))
  (:`Pressed`
    (`self.JudgeInput` 3)))

(event `self.ReceiveBeginPlay`
  (bind _asbp_third_person_character (cast `/Game/ABM/Core/Character/BP_ThirdPersonCharacter` (`GameplayStatics.GetPlayerCharacter` 0)))
  (set `self.PlayerRef` _asbp_third_person_character)
  (`self.BuildNotes`)
  (`self.EnableInput` (`GameplayStatics.GetPlayerController` 0)))

(event `TickInGame`
  (bind _widget (`self.Widget`))
  (bind _returnvalue (+ (`self.K2_GetActorLocation` (`self.PlayerRef`)) (`KismetMathLibrary.MakeVector` (* (`self.SpawnRadius`) -1.0))))
  (if (`self.bRunning`)
    (`/Engine/EditorBlueprintResources/StandardMacros.IsValid` _widget
      (:`Is Valid`
        (set `/Game/ABM/Core/Blueprints/MiniGame/Dance/WBP_DanceWidget.Score!` (`self.Score`) _widget)
        (set `/Game/ABM/Core/Blueprints/MiniGame/Dance/WBP_DanceWidget.combo!` (`self.Combo`) _widget)
        (if (not (> (- (`KismetSystemLibrary.GetGameTimeInSeconds`) (`self.StartTime`)) (`self.GameDuration`)))
          (for (_array_element _array_index) (`self.Notes`)
            (bind (_hittime _direction _bspawned _bjudged _noteactor) (break `/Game/ABM/Core/Blueprints/MiniGame/Dance/Data/ST_NoteData` _array_element))
            (if (and (not _bspawned) (<= (- _hittime (- (`KismetSystemLibrary.GetGameTimeInSeconds`) (`self.StartTime`))) (`self.LeadTime`)))
              (bind _returnvalue_2 (`|SpawnActorFromClass` "/Game/ABM/Core/Blueprints/MiniGame/Dance/BP_DanceNote.BP_DanceNote_C" (`KismetMathLibrary.MakeTransform` _returnvalue) "Undefined" "MultiplyWithRoot" null null))
              (`/Game/ABM/Core/Blueprints/MiniGame/Dance/BP_DanceNote.InitNote` _returnvalue_2 _returnvalue (`self.K2_GetActorLocation` (`self.PlayerRef`)) (`KismetSystemLibrary.GetGameTimeInSeconds`) (+ (`self.StartTime`) _hittime) _direction)
              (bind _structout (setmembers `/Game/ABM/Core/Blueprints/MiniGame/Dance/Data/ST_NoteData` :`StructRef` _array_element :`bSpawned` true :`NoteActor` _returnvalue_2))
              (`KismetArrayLibrary.Array_Set` (`self.Notes`) _array_index _structout)
              (`KismetArrayLibrary.Array_Set` (`self.ActiveNotes`) _array_index _returnvalue_2)
              (elif (and (not _bjudged) (> (- (`KismetSystemLibrary.GetGameTimeInSeconds`) (`self.StartTime`)) (+ _hittime (`self.GoodWindow`))))
                (setmembers `/Game/ABM/Core/Blueprints/MiniGame/Dance/Data/ST_NoteData` :`StructRef` _array_element :`bJudged` true)
                (`/Game/ABM/Core/Blueprints/MiniGame/Dance/WBP_DanceWidget.Miss/Good/Perfect` (`self.Widget`) "MISS" 0)
                (set `self.Combo` 0)
                (`/Engine/EditorBlueprintResources/StandardMacros.IsValid` _noteactor
                  (:`Is Valid`
                    (`self.K2_DestroyActor` _noteactor))))))
          (else
            (`self.StopMinigame`)))))))

(fn `BuildNotes`
  (locals (t :type "Float (double-precision)" :default 1.0))
  (`KismetArrayLibrary.Array_Clear` (`self.Notes`))
  (for _ (range 35)
    (bind _structout (setmembers `/Game/ABM/Core/Blueprints/MiniGame/Dance/Data/ST_NoteData` :`StructRef` (`self.ST_NoteData`) :`HitTime` (`local.t`) :`Direction` (`KismetMathLibrary.Conv_IntToByte` (`KismetMathLibrary.RandomIntegerInRange` 0 6)) :`bSpawned` false :`bJudged` false :`NoteActor` null))
    (`KismetArrayLibrary.Array_AddUnique` (`self.Notes`) _structout)
    (set `local.t` (+ (`local.t`) 0.8))))

(fn `JudgeInput`
  (params (Direc :type Byte))
  (locals (BestIndex :type Integer :default -1) (BestDelta :type "Float (double-precision)" :default 999.0))
  (bind _notes (`self.Notes`))
  (bind _score (`self.Score`))
  (bind _notes_2 (`self.Notes`))
  (bind _bestindex (`local.BestIndex`))
  (bind _widget (`self.Widget`))
  (bind _output (`|GetArrayItem` _notes_2 _bestindex))
  (bind (_hittime _direction _bspawned _bjudged _noteactor) (break `/Game/ABM/Core/Blueprints/MiniGame/Dance/Data/ST_NoteData` _output))
  (if (`self.bRunning`)
    (for _index (range (`KismetArrayLibrary.Array_Length` _notes))
      (bind (_hittime_2 _direction_2 _bspawned_2 _bjudged_2) (break `/Game/ABM/Core/Blueprints/MiniGame/Dance/Data/ST_NoteData` (`|GetArrayItem` _notes _index)))
      (if (and (== Direc _direction_2) (not _bjudged_2))
        (bind _returnvalue (`KismetMathLibrary.Abs` (- (- (`KismetSystemLibrary.GetGameTimeInSeconds`) (`self.StartTime`)) _hittime_2)))
        (if (< _returnvalue (`local.BestDelta`))
          (set `local.BestDelta` _returnvalue)
          (set `local.BestIndex` _index))))
    (if (!= (`local.BestIndex`) -1)
      (if (<= (`local.BestDelta`) (`self.GoodWindow`))
        (if (<= (`local.BestDelta`) (`self.PerfectWindow`))
          (set `self.Score` (+ _score 2))
          (`/Game/ABM/Core/Blueprints/MiniGame/Dance/WBP_DanceWidget.Miss/Good/Perfect` _widget "Perfect" 2)
          (else
            (set `self.Score` (+ _score 1))
            (`/Game/ABM/Core/Blueprints/MiniGame/Dance/WBP_DanceWidget.Miss/Good/Perfect` _widget "GOOD" 1)))
        (set `self.Combo` (+ (`self.Combo`) 1))
        (bind _structout (setmembers `/Game/ABM/Core/Blueprints/MiniGame/Dance/Data/ST_NoteData` :`StructRef` _output :`bJudged` true))
        (`KismetArrayLibrary.Array_Set` _notes_2 _bestindex _structout)
        (`/Engine/EditorBlueprintResources/StandardMacros.IsValid` _noteactor
          (:`Is Valid`
            (`self.K2_DestroyActor` _noteactor)))
        (else
          (`/Game/ABM/Core/Blueprints/MiniGame/Dance/WBP_DanceWidget.Miss/Good/Perfect` _widget "MISS" 0))))))

(fn `StartMinigame`
  (set `self.bRunning` true)
  (set `self.StartTime` (`KismetSystemLibrary.GetGameTimeInSeconds`))
  (set `self.Combo` 0)
  (set `self.Score` 0)
  (bind _returnvalue (`KismetSystemLibrary.K2_SetTimerDelegate` (`|CreateDelegate` :!event `TickInGame`) 0.02 true))
  (set `self.Handle` _returnvalue)
  (bind _returnvalue_2 (`|CreateWidget` "/Game/ABM/Core/Blueprints/MiniGame/Dance/WBP_DanceWidget.WBP_DanceWidget_C" null null))
  (bind _output_get (set `self.Widget` _returnvalue_2))
  (`UserWidget.AddToViewport` _output_get 0))

(fn `StopMinigame`
  (bind _activenotes (`self.ActiveNotes`))
  (set `self.bRunning` false)
  (`KismetSystemLibrary.K2_ClearAndInvalidateTimerHandle` (`self.Handle`))
  (for _array_element _activenotes
    (`self.K2_DestroyActor` _array_element))
  (`KismetArrayLibrary.Array_Clear` _activenotes)
  (`Widget.RemoveFromParent` (`self.Widget`))
  (set `self.Widget` null))

(fn `UserConstructionScript`)