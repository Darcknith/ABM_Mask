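; Laser hazard for the Lasers Infiltration minigame that blinks on and off and sends the player back to a respawn point on contact.
; On BeginPlay it binds to the StartLaser event of the first BP_LaserManager found, and the minigame start runs a looping timer at the supplied interval.
; A FlipFlop toggles the cylinder's visibility and query collision together.
; Overlapping BP_ThirdPersonCharacters move to the manager's RespawnLocation.
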(event `self.ReceiveBeginPlay`
  (bind _outactors (`GameplayStatics.GetAllActorsOfClass` "/Game/ABM/Core/Blueprints/MiniGame/Lasers_Infiltration/BP_LaserManager.BP_LaserManager_C"))
  (bind _output_get (set `self.BP_LaserManager` (`|GetArrayItem` _outactors)))
  (add `/Game/ABM/Core/Blueprints/MiniGame/Lasers_Infiltration/BP_LaserManager.StartLaser` _output_get (`|CreateDelegate` :!event `StartMiniGame`)))

(event `StartMiniGame`
  (params (`Laser ON/OFF Timer` :type "Float (double-precision)"))
  (`KismetSystemLibrary.K2_SetTimerDelegate` (`|CreateDelegate` :!event `Loop_ON/OFF`) `Laser ON/OFF Timer` true))

(event `Loop_ON/OFF`
  (bind _isa (`/Engine/EditorBlueprintResources/StandardMacros.FlipFlop`)
    (:`A`
      (`self.ApplyState` _isa))
    (:`B`
      (`self.ApplyState` _isa))))

(event `self.Cylinder.OnComponentBeginOverlap`
  (params (OverlappedComponent :type "PrimitiveComponent Object Reference") (OtherActor :type "Actor Object Reference") (OtherComp :type "PrimitiveComponent Object Reference") (OtherBodyIndex :type Integer) (bFromSweep :type Boolean) (SweepResult :type "HitResult Structure (by ref)"))
  (bind _asbp_third_person_character (cast `/Game/ABM/Core/Character/BP_ThirdPersonCharacter` OtherActor))
  (`self.K2_SetActorLocation` _asbp_third_person_character (`SceneComponent.K2_GetComponentLocation` (`/Game/ABM/Core/Blueprints/MiniGame/Lasers_Infiltration/BP_LaserManager.RespawnLocation` (`self.BP_LaserManager`))) false false))

(fn `ApplyState`
  (params (IsActive :type Boolean))
  (bind _cylinder (`self.Cylinder`))
  (`SceneComponent.SetVisibility` _cylinder IsActive false)
  (`PrimitiveComponent.SetCollisionEnabled` _cylinder (select `bool` IsActive :`false` "NoCollision" :`true` "QueryOnly" :!type "ECollisionEnabled Enum")))

(fn `UserConstructionScript`)