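; Parent manager Blueprint for minigames that can be triggered by a detection sphere and bounded by two cap boxes.
; When TriggerByDetection is set, any overlap calls MiniGameStartMessage, enables physics-only collision on both boxes and moves them to offsets from the actor.
; The construction script sizes the sphere and boxes and disables box collision.
; MiniGameStart and MiniGameEnd are empty events here.
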(event `self.Sphere.OnComponentBeginOverlap`
  (params (OverlappedComponent :type "PrimitiveComponent Object Reference") (OtherActor :type "Actor Object Reference") (OtherComp :type "PrimitiveComponent Object Reference") (OtherBodyIndex :type Integer) (bFromSweep :type Boolean) (SweepResult :type "HitResult Structure (by ref)"))
  (if (`self.bTriggerByDetection?`)
    (`self.SomeoneOverlap` OtherActor)))

(event `SomeoneOverlap`
  (params (ActorRef :type "Actor Object Reference"))
  (message `/Game/ABM/Core/Interfaces/BPI_MiniGame.MiniGameStart` self)
  (`self.setCollision` "PhysicsOnly")
  (`SceneComponent.K2_SetWorldLocation` (`self.FightCapBoxLeft`) (+ (`self.LeftBoxLoc`) (`self.K2_GetActorLocation`)) false false)
  (`SceneComponent.K2_SetWorldLocation` (`self.FightingCapBoxRight`) (+ (`self.RightBoxLoc`) (`self.K2_GetActorLocation`)) false false))

(event `/Game/ABM/Core/Interfaces/BPI_MiniGame.MiniGameStart`)

(event `/Game/ABM/Core/Interfaces/BPI_MiniGame.MiniGameEnd`)

(fn `setCollision`
  (params (NewType :type "ECollisionEnabled Enum" :default "NoCollision"))
  (`PrimitiveComponent.SetCollisionEnabled` (`self.FightingCapBoxRight`) NewType)
  (`PrimitiveComponent.SetCollisionEnabled` (`self.FightCapBoxLeft`) NewType))

(fn `UserConstructionScript`
  (`SphereComponent.SetSphereRadius` (`self.Sphere`) (`self.SphereRadius`) true)
  (`BoxComponent.SetBoxExtent` (`self.FightCapBoxLeft`) (`self.In Box Extent`) true)
  (`BoxComponent.SetBoxExtent` (`self.FightingCapBoxRight`) (`self.In Box Extent`) true)
  (`self.setCollision` "NoCollision"))