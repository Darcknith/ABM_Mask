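; BP_TriggerZone is a placeable audio trigger box that changes the outside state, music track or volumes when something overlaps it.
; On begin overlap, with no actor filter, BoxType selects which message goes to player 0's camera manager: Outside, Theme-derived track index, both, or a full-volume sound test.
; The construction script sizes the box from InBoxExtent and shows it in game only when IsDebug is set.
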(event `self.Box.OnComponentBeginOverlap`
  (params (OverlappedComponent :type "PrimitiveComponent Object Reference") (OtherActor :type "Actor Object Reference") (OtherComp :type "PrimitiveComponent Object Reference") (OtherBodyIndex :type Integer) (bFromSweep :type Boolean) (SweepResult :type "HitResult Structure (by ref)"))
  (switch `/Game/ABM/Core/Blueprints/Proto/E_TypeBox` (`self.BoxType`)
    (:`NewEnumerator0`
      (message `/Game/ABM/Core/Interfaces/BPI_CameraManager.setOutside` (`GameplayStatics.GetPlayerCameraManager` 0) (`self.Outside`)))
    (:`NewEnumerator1`
      (message `/Game/ABM/Core/Interfaces/BPI_CameraManager.setTrack` (`GameplayStatics.GetPlayerCameraManager` 0) (select `/Game/ABM/Core/Blueprints/Proto/E_EnviroPlace` (`self.Theme`) :`NewEnumerator1` 1 :`NewEnumerator2` 2 :`NewEnumerator3` 3 :`NewEnumerator5` 4 :`NewEnumerator6` 5)))
    (:`NewEnumerator2`
      (message `/Game/ABM/Core/Interfaces/BPI_CameraManager.setTrackAndOutside` (`GameplayStatics.GetPlayerCameraManager` 0) (`self.Outside`) (select `/Game/ABM/Core/Blueprints/Proto/E_EnviroPlace` (`self.Theme`) :`NewEnumerator1` 1 :`NewEnumerator2` 2 :`NewEnumerator3` 3 :`NewEnumerator5` 4 :`NewEnumerator6` 5)))
    (:`NewEnumerator3`
      (message `/Game/ABM/Core/Interfaces/BPI_CameraManager.setVolume` (`GameplayStatics.GetPlayerCameraManager` 0) 1.0 0.0 1.0 1.0))))

(fn `UserConstructionScript`
  (`BoxComponent.SetBoxExtent` (`self.Box`) (`self.InBoxExtent`) true)
  (`SceneComponent.SetHiddenInGame` (`self.Box`) (not (`self.bIsDebug?`)) false))