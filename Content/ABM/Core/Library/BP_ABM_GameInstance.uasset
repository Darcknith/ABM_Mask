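; Game Instance for the ABM project that holds the game's audio, ambiance, music (MX) and SFX volume settings.
; Each setter stores its value and calls UpdateVolume, while matching getters return the stored values.
; UpdateVolume passes all four volumes to player 0's camera manager through SetVolumeMessage.
; The Init and Shutdown events are empty.
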(event `self.ReceiveInit`)

(event `self.ReceiveShutdown`)

(fn `getVolumeAmbiance`
  (returns (VolumeAmbiance :type "Float (double-precision)"))
  (return (`self.VolumeAmbiance`)))

(fn `getVolumeAudio`
  (returns (VolumeAudio :type "Float (double-precision)"))
  (return (`self.VolumeAudio`)))

(fn `getVolumeMX`
  (returns (VolumeMX :type "Float (double-precision)"))
  (return (`self.VolumeMX`)))

(fn `getVolumeSFX`
  (returns (VolumeSFX :type "Float (double-precision)"))
  (return (`self.VolumeSFX`)))

(fn `setVolumeAmbiance`
  (params (VolumeAudio :type "Float (double-precision)"))
  (set `self.VolumeAmbiance` VolumeAudio)
  (`self.UpdateVolume`))

(fn `setVolumeAudio`
  (params (VolumeAudio :type "Float (double-precision)"))
  (set `self.VolumeAudio` VolumeAudio)
  (`self.UpdateVolume`))

(fn `setVolumeMX`
  (params (VolumeAudio :type "Float (double-precision)"))
  (set `self.VolumeMX` VolumeAudio)
  (`self.UpdateVolume`))

(fn `setVolumeSFX`
  (params (VolumeAudio :type "Float (double-precision)"))
  (set `self.VolumeSFX` VolumeAudio)
  (`self.UpdateVolume`))

(fn `UpdateVolume`
  (message `/Game/ABM/Core/Interfaces/BPI_CameraManager.setVolume` (`GameplayStatics.GetPlayerCameraManager` 0) (`self.VolumeAudio`) (`self.VolumeAmbiance`) (`self.VolumeSFX`) (`self.VolumeMX`)))