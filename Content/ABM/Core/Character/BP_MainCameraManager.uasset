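; BP_MainCameraManager is the main camera manager Blueprint, which here serves as a control point for FMOD audio rather than camera behavior.
; On BeginPlay it resets the Outside and Track parameters on its FMODAudio to zero.
; Custom events then set either parameter or both together, converting Track to a double.
; A VCA volume call is left unconnected, and GetMainCameraManager has no logic beyond its return.
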(event `self.ReceiveBeginPlay`
  (`FMODAudioComponent.SetParameter` (`self.FMODAudio`) "Outside" 0.0)
  (`FMODAudioComponent.SetParameter` (`self.FMODAudio`) "Track" 0.0))

(event `/Game/ABM/Core/Interfaces/BPI_CameraManager.setTrackAndOutside`
  (params (Outside :type "Float (double-precision)") (Track :type Integer))
  (`FMODAudioComponent.SetParameter` (`self.FMODAudio`) "Outside" Outside)
  (`FMODAudioComponent.SetParameter` (`self.FMODAudio`) "Track" (`KismetMathLibrary.Conv_IntToDouble` Track)))

(event `/Game/ABM/Core/Interfaces/BPI_CameraManager.setOutside`
  (params (Outside :type "Float (double-precision)"))
  (`FMODAudioComponent.SetParameter` (`self.FMODAudio`) "Outside" Outside))

(event `/Game/ABM/Core/Interfaces/BPI_CameraManager.setTrack`
  (params (Track :type Integer))
  (`FMODAudioComponent.SetParameter` (`self.FMODAudio`) "Track" (`KismetMathLibrary.Conv_IntToDouble` Track)))

(fn `getMainCameraManager`
  (returns (CameraManagerRef :type "/Game/ABM/Core/Character/BP_MainCameraManager Object Reference"))
  (return null))

(fn `UserConstructionScript`)