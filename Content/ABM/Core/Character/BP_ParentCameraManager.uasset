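; Parent camera manager Blueprint that, in the graphs shown, controls the game's FMOD music and ambience parameters and mix volumes.
; BeginPlay zeroes the Outside and Track parameters, then sets Ambiance, SFX and MX VCAs from GameInstance volumes, with Ambiance using master volume squared.
; Events update either parameter or both, printing Track changes, while SetVolume scales each VCA by master volume.
; GetMainCameraManager is an empty stub.
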(event `self.ReceiveBeginPlay`
  (bind _gameinstance (`/Game/ABM/Core/Library/BFL_ABM.GetABMGameInstance`))
  (bind _volumeaudio (`/Game/ABM/Core/Library/BP_ABM_GameInstance.getVolumeAudio` _gameinstance))
  (`FMODAudioComponent.SetParameter` (`self.FMODAudio`) "Outside" 0.0)
  (`FMODAudioComponent.SetParameter` (`self.FMODAudio`) "Track" 0.0)
  (`FMODBlueprintStatics.VCASetVolume` (`self.VCA_Ambiance`) (* _volumeaudio (`/Game/ABM/Core/Library/BP_ABM_GameInstance.getVolumeAudio` _gameinstance)))
  (`FMODBlueprintStatics.VCASetVolume` (`self.VCA_SFX`) (* _volumeaudio (`/Game/ABM/Core/Library/BP_ABM_GameInstance.getVolumeSFX` _gameinstance)))
  (`FMODBlueprintStatics.VCASetVolume` (`self.VCA_MX`) (* _volumeaudio (`/Game/ABM/Core/Library/BP_ABM_GameInstance.getVolumeMX` _gameinstance))))

(event `self.setTrackAndOutside`
  (params (Outside :type "Float (double-precision)") (Track :type Integer))
  (bind _returnvalue (`KismetMathLibrary.Conv_IntToDouble` Track))
  (`FMODAudioComponent.SetParameter` (`self.FMODAudio`) "Outside" Outside)
  (`FMODAudioComponent.SetParameter` (`self.FMODAudio`) "Track" _returnvalue)
  (`KismetSystemLibrary.PrintString` (`KismetStringLibrary.Conv_DoubleToString` _returnvalue)))

(event `self.setOutside`
  (params (Outside :type "Float (double-precision)"))
  (`FMODAudioComponent.SetParameter` (`self.FMODAudio`) "Outside" Outside))

(event `self.setTrack`
  (params (Track :type Integer))
  (bind _returnvalue (`KismetMathLibrary.Conv_IntToDouble` Track))
  (`FMODAudioComponent.SetParameter` (`self.FMODAudio`) "Track" _returnvalue)
  (`KismetSystemLibrary.PrintString` (`KismetStringLibrary.Conv_DoubleToString` _returnvalue)))

(event `self.setVolume`
  (params (setAudio :type "Float (double-precision)") (setAmbience :type "Float (double-precision)") (setSFX :type "Float (double-precision)") (setMX :type "Float (double-precision)"))
  (`FMODBlueprintStatics.VCASetVolume` (`self.VCA_Ambiance`) (* setAudio setAmbience))
  (`FMODBlueprintStatics.VCASetVolume` (`self.VCA_SFX`) (* setAudio setSFX))
  (`FMODBlueprintStatics.VCASetVolume` (`self.VCA_MX`) (* setAudio setMX)))

(fn `getMainCameraManager`
  (returns (CameraManagerRef :type "/Game/ABM/Core/Character/BP_MainCameraManager Object Reference"))
  (return null))

(fn `UserConstructionScript`)