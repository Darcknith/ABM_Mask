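; BP_AC_MaskState is an actor component that stores the current mask state of its owner in the mask system.
; SetMask ignores unchanged values, otherwise records the old mask, updates the visual, fires OnMaskChanged and reports whether it changed.
; The visual step swaps the owning BP_ThirdPersonCharacter's skeletal mesh using a mask-to-mesh map.
; HasMask matches the current mask, with one enum value passing every check.
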(fn `ApplyVisual`
  (params (Mask :type "/Game/ABM/Mask_System/Add_Component/E_MaskState Enum" :default "NewEnumerator0"))
  (bind (_value _returnvalue) (`BlueprintMapLibrary.Map_Find` (`self.MaskStateToVisual`) (`local.Mask`)))
  (bind _asbp_third_person_character (cast `/Game/ABM/BP_ThirdPersonCharacter` (`self.GetOwner`))
    (:`then`
      (if _returnvalue
        (`SkeletalMeshComponent.SetSkeletalMeshAsset` (`Character.Mesh` _asbp_third_person_character) _value)
        (return)
        (else
          (return))))
    (:`CastFailed`
      (return))))

(fn `GetMask`
  (returns (CurrentMask :type "/Game/ABM/Mask_System/Add_Component/E_MaskState Enum"))
  (return (`self.CurrentMask`)))

(fn `HasMask`
  (params (MaskToCheck :type "/Game/ABM/Mask_System/Add_Component/E_MaskState Enum" :default "NewEnumerator0"))
  (returns (`HasMask?` :type Boolean))
  (bind _currentmask (`self.CurrentMask`))
  (return (or (`|EnumEquality` MaskToCheck _currentmask) (`|EnumEquality` _currentmask "NewEnumerator5"))))

(fn `SetMask`
  (params (NewMask :type "/Game/ABM/Mask_System/Add_Component/E_MaskState Enum" :default "NewEnumerator0"))
  (returns (bDidChange :type Boolean))
  (locals (OldMask :type "/Game/ABM/Mask_System/Add_Component/E_MaskState Enum" :default "NewEnumerator0"))
  (if (`|EnumInequality` NewMask (`self.CurrentMask`))
    (set `local.OldMask` (`self.CurrentMask`))
    (bind _output_get (set `self.CurrentMask` (`local.NewMask`)))
    (`self.ApplyVisual` _output_get)
    (`self.OnMaskChanged` (`local.OldMask`) (`self.CurrentMask`))
    (return true)
    (else
      (return false))))