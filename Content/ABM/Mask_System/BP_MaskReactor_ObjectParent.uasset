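; Base actor for world objects that react to which mask the player has, with empty events for visuals and activation left to children.
; On BeginPlay it gets player 0's mask component through BPI_MaskOwner and optionally listens for mask changes.
; UpdateRequirement checks the required mask, then broadcasts and calls the satisfied or unsatisfied visual event only when the state flips.
; TryActivate fires a success or failure event based on that cached state.
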(event `self.ReceiveBeginPlay`
  (`self.InitializeWithPlayer` (`GameplayStatics.GetPlayerCharacter` 0)))

(event `ApplySatisfiedVisual`)

(event `ApplyUnsitisfiedVisual`)

(event `OnActivatedSucces`
  (params (Investigator :type "Actor Object Reference")))

(event `OnActivatedFailed`
  (params (Investigator :type "Actor Object Reference")))

(event `OnPlayerMaskChanged_Bound`
  (params (OldMask :type "/Game/ABM/Mask_System/Add_Component/E_MaskState Enum" :default "NewEnumerator0") (NewMask :type "/Game/ABM/Mask_System/Add_Component/E_MaskState Enum" :default "NewEnumerator0"))
  (`self.UpdateRequirement`))

(fn `CanActivate`
  (returns (`CanActivate?` :type Boolean))
  (return (`self.bIsSatisfied`)))

(fn `InitializeWithPlayer`
  (params (PlayerActor :type "Actor Object Reference"))
  (bind _cachedmaskcomp (`self.CachedMaskComp`))
  (bind _output_get (set `self.CachedPlayer` PlayerActor))
  (if (`KismetSystemLibrary.DoesImplementInterface` _output_get "/Game/ABM/Mask_System/Add_Component/BPI_MaskOwner.BPI_MaskOwner_C")
    (bind _bp_ac_maskstate (message `/Game/ABM/Mask_System/Add_Component/BPI_MaskOwner.GetMaskComponent` (`local.PlayerActor`)))
    (set `self.CachedMaskComp` _bp_ac_maskstate)
    (`self.UpdateRequirement`)
    (if (`self.bAutoListenPlayerMask`)
      (if (`KismetSystemLibrary.IsValid` _cachedmaskcomp)
        (add `/Game/ABM/Mask_System/Add_Component/BP_AC_MaskState.OnMaskChanged` _cachedmaskcomp (`|CreateDelegate` :!event `OnPlayerMaskChanged_Bound`))
        (return)
        (else
          (return)))
      (else
        (return)))
    (else
      (`self.UpdateRequirement`)
      (return))))

(fn `TryActivate`
  (params (Investigator :type "Actor Object Reference"))
  (bind _canactivate_ (`self.CanActivate`))
  (if _canactivate_
    (`self.OnActivatedSucces` (`local.Investigator`))
    (return)
    (else
      (`self.OnActivatedFailed` (`local.Investigator`))
      (return))))

(fn `UpdateRequirement`
  (locals (bNowSatisfied :type Boolean :default false))
  (bind _cachedmaskcomp (`self.CachedMaskComp`))
  (bind _bnowsatisfied (`local.bNowSatisfied`))
  (if (`KismetSystemLibrary.IsValid` _cachedmaskcomp)
    (bind _hasmask_ (`/Game/ABM/Mask_System/Add_Component/BP_AC_MaskState.HasMask` _cachedmaskcomp (`self.RequiredMask`)))
    (bind _output_get (set `local.bNowSatisfied` _hasmask_))
    (if (!= _output_get (`self.bIsSatisfied`))
      (set `self.bIsSatisfied` _bnowsatisfied)
      (`self.OnRequirementChanged_Object` _bnowsatisfied)
      (if (`local.bNowSatisfied`)
        (`self.ApplySatisfiedVisual`)
        (return)
        (else
          (`self.ApplyUnsitisfiedVisual`)
          (return)))
      (else
        (return)))
    (else
      (return))))

(fn `UserConstructionScript`)