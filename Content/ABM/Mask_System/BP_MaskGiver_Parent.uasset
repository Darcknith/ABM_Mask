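; BP_MaskGiver_Parent is a base actor that hands a configured mask to a receiver.
; TryGiveMask checks that the receiver implements BPI_MaskOwner, fetches its mask component through the interface and calls SetMask with MaskToGive.
; On success it fires the empty OnGiven event and destroys itself if DestroyOnSpawn is set.
; The parent has no trigger logic of its own, as nothing in it calls TryGiveMask.
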(event `Event OnGiven`
  (params (Reciver :type "Actor Object Reference")))

(fn `TryGiveMask`
  (params (Reciver :type "Actor Object Reference"))
  (if (`KismetSystemLibrary.DoesImplementInterface` Reciver "/Game/ABM/Mask_System/Add_Component/BPI_MaskOwner.BPI_MaskOwner_C")
    (bind _bp_ac_maskstate (message `/Game/ABM/Mask_System/Add_Component/BPI_MaskOwner.GetMaskComponent` (`local.Reciver`)))
    (if (`KismetSystemLibrary.IsValid` _bp_ac_maskstate)
      (bind _bdidchange (`/Game/ABM/Mask_System/Add_Component/BP_AC_MaskState.SetMask` _bp_ac_maskstate (`self.MaskToGive`)))
      (if _bdidchange
        (`self.Event OnGiven` (`local.Reciver`))
        (if (`self.DestroyOnSpawn`)
          (`self.K2_DestroyActor`))
        (else
          (return))))))

(fn `UserConstructionScript`)